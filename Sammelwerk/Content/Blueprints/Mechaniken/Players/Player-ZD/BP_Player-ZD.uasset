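; Player Blueprint that registers the IMC_Player Enhanced Input mapping context on its player controller at BeginPlay.
; A PlayerTickDamage event waits a second, then subtracts zero from Leben (health), so it changes nothing.
; An unconnected chain holds hit sounds, a camera fade and a level load on a Leben check, plus the only call to PlayerTickDamage, so none of it runs.
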(event `self.ReceiveBeginPlay`
  (bind _asplayer_controller (cast `PlayerController` (`self.GetController`)))
  (`EnhancedInputSubsystemInterface.AddMappingContext` (pcsubsystem `EnhancedInputLocalPlayerSubsystem` _asplayer_controller) "/Game/Blueprints/Funktionen/Input/IMC_Player.IMC_Player" 0 (struct)))

(event `PlayerTickDamage`
  (`KismetSystemLibrary.Delay` 1.0)
  (set `self.Leben` (- (`self.Leben`) 0.0)))

(fn `UserConstructionScript`)