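; BP_SequenceAuslöser is a trigger actor that fires when an actor implementing BPI_PickupActor overlaps its Box.
; A timeline slides the Box slightly along local Y, then plays the assigned LevelSequence once and sends an on message to ActorsToTrigger via BPI_Trigger.
; A backward finish would send off, but nothing in this graph reverses the timeline.
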(event `self.Box.OnComponentBeginOverlap`
  (params (OverlappedComponent :type "PrimitiveComponent Object Reference") (OtherActor :type "Actor Object Reference") (OtherComp :type "PrimitiveComponent Object Reference") (OtherBodyIndex :type Integer) (bFromSweep :type Boolean) (SweepResult :type "HitResult Structure (by ref)"))
  (bind _level_sequence (`self.Level Sequence`))
  (if (`KismetSystemLibrary.DoesImplementInterface` OtherActor "/Game/Blueprints/Funktionen/Interface/BPI_PickupActor.BPI_PickupActor_C")
    (bind (_direction _alpha) (`Timeline|Zeitleiste`)
      (:`Update`
        (`SceneComponent.K2_SetRelativeLocation` (`self.Box`) (`KismetMathLibrary.VLerp` (0.0 0.0 0.0) (0.0 -6.0 0.0) _alpha) false false))
      (:`Finished`
        (switch `ETimelineDirection` _direction
          (:`Forward`
            (`|ExecutionSequence`
              (:`then_0`
                ; Player LevelSequence
                (`/Engine/EditorBlueprintResources/StandardMacros.DoOnce` false
                  (:`Completed`
                    (`/Engine/EditorBlueprintResources/StandardMacros.IsValid` _level_sequence
                      (:`Is Valid`
                        (`MovieSceneSequencePlayer.Play` (`LevelSequenceActor.SequencePlayer` _level_sequence)))))))
              (:`then_1`
                ; Trigger Loop On
                (for _array_element (`self.ActorsToTrigger`)
                  (if (`KismetSystemLibrary.DoesImplementInterface` _array_element "/Game/Blueprints/Funktionen/Interface/BPI_Trigger.BPI_Trigger_C")
                    (message `/Game/Blueprints/Funktionen/Interface/BPI_Trigger.Trigger` _array_element true null))))))
          (:`Backward`
            ; Trigger Loop Off
            (for _array_element_2 (`self.ActorsToTrigger`)
              (if (`KismetSystemLibrary.DoesImplementInterface` _array_element_2 "/Game/Blueprints/Funktionen/Interface/BPI_Trigger.BPI_Trigger_C")
                (message `/Game/Blueprints/Funktionen/Interface/BPI_Trigger.Trigger` _array_element_2 false null)))))))))

(fn `UserConstructionScript`)