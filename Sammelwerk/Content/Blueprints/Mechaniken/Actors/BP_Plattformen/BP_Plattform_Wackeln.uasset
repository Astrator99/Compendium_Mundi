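; Wobbling platform Blueprint (Plattform-Wackeln) that shakes the whole actor when its CEPlayAnimation event runs.
; The shake is hand-scripted as a short chain of small local offsets separated by brief delays, without sweep or timeline.
; The offsets do not fully cancel, so each run leaves the actor slightly displaced.
; It finishes by calling CEResetDoOnce; BeginPlay is disabled and the construction script only calls its parent.
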(event `self.CE_PlayAnimation`
  ;[0 1 0 0.5] CE_PlayAnimation: Plattform-Wackeln
  (`self.K2_AddActorLocalOffset` (0.0 0.0 -3.0))
  (`KismetSystemLibrary.Delay` 0.05)
  (`self.K2_AddActorLocalOffset` (-2.0 0.0 2.0))
  (`KismetSystemLibrary.Delay` 0.05)
  (`self.K2_AddActorLocalOffset` (3.0 -2.0 0.0))
  (`KismetSystemLibrary.Delay` 0.05)
  (`self.K2_AddActorLocalOffset` (-5.0 0.0 -1.0))
  (`KismetSystemLibrary.Delay` 0.05)
  (`self.K2_AddActorLocalOffset` (5.0 -3.0 2.0))
  (`KismetSystemLibrary.Delay` 0.05)
  (`self.K2_AddActorLocalOffset` (1.0 5.0 1.0))
  (`KismetSystemLibrary.Delay` 0.05)
  (`self.CE_ResetDoOnce`))

(fn `UserConstructionScript`
  (`parent.UserConstructionScript`))