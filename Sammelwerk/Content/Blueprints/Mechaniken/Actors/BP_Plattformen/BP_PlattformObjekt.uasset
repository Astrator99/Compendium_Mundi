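; Base-style platform object actor that reacts when a player-management actor (BPI_PlayerManagement) enters its trigger area.
; The first valid overlap plays a 2D sound and calls a play-animation event through a DoOnce gate, which CE_ResetDoOnce re-arms.
; CE_PlayAnimation is an empty hook here, and BeginPlay caches the actor's scale.
; Reaktion toggles collision and visibility together from one boolean.
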(event `self.ReceiveBeginPlay`
  (set `self.Größe Actors` (`self.GetActorScale3D`)))

(event `self.TriggerBereich.OnComponentBeginOverlap`
  (params (OverlappedComponent :type "PrimitiveComponent Object Reference") (OtherActor :type "Actor Object Reference") (OtherComp :type "PrimitiveComponent Object Reference") (OtherBodyIndex :type Integer) (bFromSweep :type Boolean) (SweepResult :type "HitResult Structure (by ref)"))
  (if (`KismetSystemLibrary.DoesImplementInterface` OtherActor "/Game/Blueprints/Funktionen/Interface/BPI_PlayerManagement.BPI_PlayerManagement_C")
    (`/Engine/EditorBlueprintResources/StandardMacros.DoOnce` false :!label _label
      (:`Completed`
        (`GameplayStatics.SpawnSound2D` null 1.0 1.0 0.0 null)
        (`self.CE_PlayAnimation`)))))

(event `CE_ResetDoOnce`
  (goto _label :!via `Reset`))

(event `CE_PlayAnimation`)

(event `Reaktion`
  (params (`Hat Kollision` :type Boolean))
  (`self.SetActorEnableCollision` `Hat Kollision`)
  (`self.SetActorHiddenInGame` (not `Hat Kollision`)))

(fn `UserConstructionScript`)