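; Anomaly platform child Blueprint that scales itself along a timeline, turns off its collision and respawns after a delay.
; CEPlayAnimation plays a timeline, sized to a configurable duration, whose alpha multiplies the actor's base scale.
; One Finished branch uses playback position to tell directions apart: the forward end disables collision and reverses after the delay, while the reverse end restores collision and calls CEResetDoOnce.
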(event `self.ReceiveBeginPlay`
  (`parent.ReceiveBeginPlay`)
  (`TimelineComponent.SetTimelineLength` (`self.Zeitleiste`) (`self.Zeitdauer`)))

(event `self.CE_PlayAnimation`
  (bind (_direction _alpha) (`Timeline|Zeitleiste` :!via `PlayFromStart` :!label _label)
    (:`Update`
      (`self.SetActorScale3D` (* _alpha (`self.Größe Actors`))))
    (:`Finished`
      (if (> (`TimelineComponent.GetPlaybackPosition` (`self.Zeitleiste`)) 0.1)
        (`self.SetActorEnableCollision` false)
        (`KismetSystemLibrary.Delay` (`self.Respawndauer`))
        (goto _label :!via `Reverse`)
        (else
          (`self.SetActorEnableCollision` true)
          (`self.CE_ResetDoOnce`))))))

(fn `UserConstructionScript`
  (`parent.UserConstructionScript`))