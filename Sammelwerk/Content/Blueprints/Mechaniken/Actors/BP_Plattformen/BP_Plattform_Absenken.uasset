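; BP_Plattform_Absenken is a platform child Blueprint that lowers vertically and returns when the trigger overlap ends.
; On BeginPlay it stores the root's relative location and sets the timeline length from Zeitdauer.
; CEPlayAnimation plays the timeline, lerping the root from its start toward a Z offset of AbsenkTiefe.
; Ending overlap with TriggerBereich calls CEResetDoOnce and reverses the timeline from its current position.
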(event `self.ReceiveBeginPlay`
  (`parent.ReceiveBeginPlay`)
  (set `self.StartLocation` (`SceneComponent.RelativeLocation` (`self.DefaultSceneRoot`)))
  (`TimelineComponent.SetTimelineLength` (`self.TL_Absenken`) (`self.Zeitdauer`)))

(event `self.CE_PlayAnimation`
  (bind _startlocation (`self.StartLocation`))
  (bind (_direction _alpha) (`Timeline|TL_Absenken` :!label _label)
    (:`Update`
      (`SceneComponent.K2_SetRelativeLocation` (`self.DefaultSceneRoot`) (`KismetMathLibrary.VLerp` _startlocation (+ _startlocation (`KismetMathLibrary.MakeVector` 0.0 0.0 (`self.AbsenkTiefe`))) _alpha) false false))))

(event `self.TriggerBereich.OnComponentEndOverlap`
  (params (OverlappedComponent :type "PrimitiveComponent Object Reference") (OtherActor :type "Actor Object Reference") (OtherComp :type "PrimitiveComponent Object Reference") (OtherBodyIndex :type Integer))
  (`self.CE_ResetDoOnce`)
  (goto _label :!via `Reverse`))

(fn `UserConstructionScript`
  (`parent.UserConstructionScript`))