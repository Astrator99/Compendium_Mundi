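; BP_Plattform_Falle is a trap platform that drops away when CEPlayAnimation is called, moving its 3D and 2D fall objects.
; With NutzeEchtePhysik set, both simulate physics, overlap Pawns and the actor is destroyed after a delay.
; Otherwise, timeline TL_Absturz lerps their relative location by AbsenkTiefe along Z and their rotation.
; It also drives the sprite's opacity, then hides the actor in game without destroying it.
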(event `self.CE_PlayAnimation`
  (bind _startlocation (`self.StartLocation`))
  ;[0.15 0 0.005778 0.5] Falle: Physik- oder Animationsabsturz
  (if (`self.NutzeEchtePhysik`)
    (`PrimitiveComponent.SetSimulatePhysics` (`self.Fallobjekt 3D`) true)
    (`PrimitiveComponent.SetSimulatePhysics` (`self.Fallobjekt 2D`) true)
    (`PrimitiveComponent.SetCollisionResponseToChannel` (`self.Fallobjekt 3D`) "ECC_Pawn" "ECR_Overlap")
    (`PrimitiveComponent.SetCollisionResponseToChannel` (`self.Fallobjekt 2D`) "ECC_Pawn" "ECR_Overlap")
    (`KismetSystemLibrary.Delay` 3.0)
    (`self.K2_DestroyActor`)
    (else
      (bind (_direction _alpha _sichtbarkeit) (`Timeline|TL_Absturz` :!via `PlayFromStart`)
        (:`Update`
          (`SceneComponent.K2_SetRelativeLocationAndRotation` (`self.Fallobjekt 3D`) (`KismetMathLibrary.VLerp` _startlocation (+ _startlocation (`KismetMathLibrary.MakeVector` 0.0 0.0 (`self.AbsenkTiefe`))) _alpha) (`KismetMathLibrary.RLerp` (struct) (struct :`Yaw` 180.0) _alpha) false false)
          (`SceneComponent.K2_SetRelativeLocationAndRotation` (`self.Fallobjekt 2D`) (`KismetMathLibrary.VLerp` _startlocation (+ _startlocation (`KismetMathLibrary.MakeVector` 0.0 0.0 (`self.AbsenkTiefe`))) _alpha) (`KismetMathLibrary.RLerp` (struct) (struct :`Yaw` 180.0) _alpha) false false)
          (`PaperSpriteComponent.SetSpriteColor` (`self.Fallobjekt 2D`) (make `LinearColor` 1.0 1.0 1.0 _sichtbarkeit)))
        (:`Finished`
          (`self.SetActorHiddenInGame` true))))))

(fn `UserConstructionScript`
  (`parent.UserConstructionScript`))