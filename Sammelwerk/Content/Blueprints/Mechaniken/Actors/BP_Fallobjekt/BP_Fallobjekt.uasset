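; BP_Fallobjekt is a temporary platform that vanishes after an actor implementing BPI_Trigger enters its trigger, then respawns.
; A DoOnce-gated overlap plays a sound, waits, hides the platform, waits again, restores it and re-arms the trigger.
; A timeline scales the actor relative to its initial size, disabling collision and visibility when finished forward.
; Respawning re-enables both before playing the timeline in reverse.
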(event `self.ReceiveBeginPlay`
  (set `self.Größe Actors` (`self.GetActorScale3D`)))

(event `self.TriggerBereich.OnComponentBeginOverlap`
  (params (OverlappedComponent :type "PrimitiveComponent Object Reference") (OtherActor :type "Actor Object Reference") (OtherComp :type "PrimitiveComponent Object Reference") (OtherBodyIndex :type Integer) (bFromSweep :type Boolean) (SweepResult :type "HitResult Structure (by ref)"))
  (if (`KismetSystemLibrary.DoesImplementInterface` OtherActor "/Game/Blueprints/Funktionen/Interface/BPI_Trigger.BPI_Trigger_C")
    (`/Engine/EditorBlueprintResources/StandardMacros.DoOnce` false :!label _label
      (:`Completed`
        (`GameplayStatics.SpawnSound2D` null 1.0 1.0 0.0 null)
        (`KismetSystemLibrary.Delay` (`self.Zeitdauer`))
        (`self.Animierte Plattform` false)
        (`KismetSystemLibrary.Delay` (`self.Respawndauer`))
        (`self.Animierte Plattform` true)
        (`self.Reset`)))))

(event `Reset`
  (goto _label :!via `Reset`))

(event `Animierte Plattform`
  (params (Sichtbar :type Boolean))
  (if (not Sichtbar)
    (bind (_direction _alpha) (`Timeline|Zeitleiste` :!label _label_2)
      (:`Update`
        (`self.SetActorScale3D` (* _alpha (`self.Größe Actors`))))
      (:`Finished`
        (switch `ETimelineDirection` _direction
          (:`Forward`
            (`self.Reaktion` false)))))
    (else
      (`self.Reaktion` true)
      (goto _label_2 :!via `Reverse`))))

(event `Reaktion`
  (params (`Hat Kollision` :type Boolean))
  (`self.SetActorEnableCollision` `Hat Kollision`)
  (`self.SetActorHiddenInGame` (not `Hat Kollision`)))

(fn `UserConstructionScript`)