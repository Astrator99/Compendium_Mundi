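; Level goal actor that ends the current level when the player reaches it and loads the level set in LevelName.
; A sphere overlap accepts either BP_Player or BP_Player-ZD and disables that character's movement.
; Both branches merge into a DoOnce that starts a held camera fade-out and opens the level after a delay shorter than the fade.
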(event `self.Sphere.OnComponentBeginOverlap`
  (params (OverlappedComponent :type "PrimitiveComponent Object Reference") (OtherActor :type "Actor Object Reference") (OtherComp :type "PrimitiveComponent Object Reference") (OtherBodyIndex :type Integer) (bFromSweep :type Boolean) (SweepResult :type "HitResult Structure (by ref)"))
  (bind _asbp_player (cast `/Game/Blueprints/Mechaniken/Players/Player-3D/BP_Player` OtherActor)
    (:`then`
      (`CharacterMovementComponent.DisableMovement` (`Character.CharacterMovement` _asbp_player)))
    (:`CastFailed`
      (bind _asbp_player__zd (cast `/Game/Blueprints/Mechaniken/Players/Player-ZD/BP_Player-ZD` OtherActor))
      (`CharacterMovementComponent.DisableMovement` (`Character.CharacterMovement` _asbp_player__zd))))
  (`/Engine/EditorBlueprintResources/StandardMacros.DoOnce` false
    (:`Completed`
      (`PlayerCameraManager.StartCameraFade` :`self` (`GameplayStatics.GetPlayerCameraManager` 0) :`ToAlpha` 1.0 :`Duration` 2.0 :`bHoldWhenFinished` true)
      (`KismetSystemLibrary.Delay` 1.0)
      (`GameplayStatics.OpenLevelBySoftObjectPtr` (`self.Level Name`)))))

(fn `UserConstructionScript`)