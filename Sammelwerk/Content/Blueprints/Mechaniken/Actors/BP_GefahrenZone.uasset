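; BP_GefahrenZone is a hazard zone actor that kills or damages players entering its Todeszone trigger.
; On overlap, actors implementing BPI_PlayerManagement are handled by FallenTyp: instant death through the GameMode, one-time damage, or interval damage.
; Damage runs through messages to the player, and instant death and single hits also play a 2D hit sound.
; Leaving the trigger sends the stop message for damage over time, regardless of trap type.
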(event `self.Todeszone.OnComponentBeginOverlap`
  (params (OverlappedComponent :type "PrimitiveComponent Object Reference") (OtherActor :type "Actor Object Reference") (OtherComp :type "PrimitiveComponent Object Reference") (OtherBodyIndex :type Integer) (bFromSweep :type Boolean) (SweepResult :type "HitResult Structure (by ref)"))
  (if (`KismetSystemLibrary.DoesImplementInterface` OtherActor "/Game/Blueprints/Funktionen/Interface/BPI_PlayerManagement.BPI_PlayerManagement_C")
    (set `self.GetroffenerSpieler` OtherActor)
    (switch `/Game/Blueprints/Funktionen/Enumeration/E_FallenTypen` (`self.FallenTyp`)
      (:`NewEnumerator0`
        (message `/Game/Blueprints/Funktionen/Interface/BPI_GameManagement.TriggerPlayerDeath` (`GameplayStatics.GetGameMode`) OtherActor)
        (`GameplayStatics.PlaySound2D` "/Game/Assets-Audio/Sounds/Sound_Hit2.Sound_Hit2" 1.0 1.0 0.0 null null))
      (:`NewEnumerator1`
        (message `/Game/Blueprints/Funktionen/Interface/BPI_PlayerManagement.ApplyDamage` OtherActor (`self.SchadensMenge`))
        (`GameplayStatics.PlaySound2D` "/Game/Assets-Audio/Sounds/Sound_Hit2.Sound_Hit2" 1.0 1.0 0.0 null null))
      (:`NewEnumerator2`
        (message `/Game/Blueprints/Funktionen/Interface/BPI_PlayerManagement.StartDamageOverTime` OtherActor (`self.SchadensIntervall`) (`self.SchadensMenge`))))))

(event `self.Todeszone.OnComponentEndOverlap`
  (params (OverlappedComponent :type "PrimitiveComponent Object Reference") (OtherActor :type "Actor Object Reference") (OtherComp :type "PrimitiveComponent Object Reference") (OtherBodyIndex :type Integer))
  (message `/Game/Blueprints/Funktionen/Interface/BPI_PlayerManagement.StopDamageOverTime` OtherActor))

(fn `UserConstructionScript`)