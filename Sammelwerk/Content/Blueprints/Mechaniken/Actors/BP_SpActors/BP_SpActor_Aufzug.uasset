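; BP_SpActor_Aufzug is an interactable elevator actor that runs one timed, alternating cycle per interaction.
; Interact ignores calls while FährtAktuell is set, and a FlipFlop toggles the Gradeaus direction flag on each accepted use.
; After a WarteZeit delay it raises AlleRichtungen for another WarteZeit, then clears it and unlocks.
; The graph only sets state flags and contains no movement code.
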(event `/Game/Blueprints/Funktionen/Interface/BPI_PlayerManagement.Interact`
  (if (not (`self.FährtAktuell?`))
    (set `self.FährtAktuell?` true)
    (`/Engine/EditorBlueprintResources/StandardMacros.FlipFlop`
      (:`A`
        (set `self.Gradeaus` true))
      (:`B`
        (set `self.Gradeaus` false)))
    (`KismetSystemLibrary.Delay` (`self.WarteZeit`))
    (set `self.Alle Richtungen` true)
    (`KismetSystemLibrary.Delay` (`self.WarteZeit`))
    (set `self.Alle Richtungen` false)
    (set `self.FährtAktuell?` false)))

(fn `UserConstructionScript`
  (`parent.UserConstructionScript`))