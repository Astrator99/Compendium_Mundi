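; BP_Deathzone is a hazard volume that triggers player death and respawn when its Todeszone component is overlapped.
; The overlapping actor must cast to GM_Game, on which it calls PlayerDeath.
; It then disables player movement, plays a hit sound, fades the camera out and calls PlayerRespawn after a short delay.
; An alternative sequence that destroys an actor is left unconnected.
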(event `self.Todeszone.OnComponentBeginOverlap`
  (params (OverlappedComponent :type "PrimitiveComponent Object Reference") (OtherActor :type "Actor Object Reference") (OtherComp :type "PrimitiveComponent Object Reference") (OtherBodyIndex :type Integer) (bFromSweep :type Boolean) (SweepResult :type "HitResult Structure (by ref)"))
  (bind _asgm_game (cast `/Game/Blueprints/GM_Game` OtherActor))
  (`/Game/Blueprints/GM_Game.PlayerDeath` _asgm_game)
  (`CharacterMovementComponent.DisableMovement` (`Character.CharacterMovement` (`GameplayStatics.GetPlayerCharacter` 0)))
  (`GameplayStatics.PlaySound2D` "/Game/Assets-Audio/Sounds/Sound_Hit.Sound_Hit" 1.0 1.0 0.0 null null)
  (`PlayerCameraManager.StartCameraFade` :`self` (`GameplayStatics.GetPlayerCameraManager` 0) :`FromAlpha` 0.5 :`ToAlpha` 1.0 :`Duration` 1.0 :`bHoldWhenFinished` true)
  (`KismetSystemLibrary.Delay` 1.0)
  (`/Game/Blueprints/GM_Game.PlayerRespawn` _asgm_game))

(fn `UserConstructionScript`)