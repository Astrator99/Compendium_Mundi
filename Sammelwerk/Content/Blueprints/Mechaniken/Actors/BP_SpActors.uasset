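; Moving platform actor that travels along the spline of a referenced BPSpline at a set speed while switched on through its Trigger event.
; Every Tick it places itself at the current spline distance, then advances or reduces that distance by speed times delta time.
; At the far end it waits, then restarts (Loop) or reverses, or stops if one-way (EinWeg).
; Back at the start it reverses without waiting.
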(event `self.ReceiveTick`
  (params (DeltaSeconds :type "Float (single-precision)"))
  (`self.Move Plattform`))

(event `Event Trigger`
  (params (On :type Boolean))
  (set `self.Alle Richtungen` On))

(event `Update Position`
  (`self.K2_SetActorLocation` (`SplineComponent.GetLocationAtDistanceAlongSpline` (`/Game/Blueprints/Mechaniken/Actors/BP_Spline.Spline` (`self.BP Spline`)) (`self.Entfernung zum Spline`) "World")))

(event `Move Plattform`
  (if (`self.Alle Richtungen`)
    (`/Engine/EditorBlueprintResources/StandardMacros.IsValid` (`self.BP Spline`)
      (:`Is Valid`
        (`|ExecutionSequence`
          (:`then_0`
            (`self.Update Position`))
          (:`then_1`
            (if (`self.Gradeaus`)
              (if (< (`self.Entfernung zum Spline`) (`SplineComponent.GetSplineLength` (`/Game/Blueprints/Mechaniken/Actors/BP_Spline.Spline` (`self.BP Spline`))))
                ;[0.007938 0.2 0.01045 0.5] Distanz aufwärts zählen
                (set `self.Entfernung zum Spline` (+ (`self.Entfernung zum Spline`) (* (`self.Geschwindigkeit`) (`GameplayStatics.GetWorldDeltaSeconds`))))
                (elif (`self.Loop`)
                  (`KismetSystemLibrary.Delay` (`self.WarteZeit`))
                  (set `self.Entfernung zum Spline` 0.0)
                  (elif (not (`self.Ein Weg`))
                    (`KismetSystemLibrary.Delay` (`self.WarteZeit`))
                    (set `self.Gradeaus` false))))
              (else
                ;[0.008023 0.2016 0.01033 0.502] Plattform nach hinten bewegen
                (if (> (`self.Entfernung zum Spline`) 0.0)
                  (set `self.Entfernung zum Spline` (- (`self.Entfernung zum Spline`) (* (`self.Geschwindigkeit`) (`GameplayStatics.GetWorldDeltaSeconds`))))
                  (elif (not (`self.Ein Weg`))
                    (set `self.Gradeaus` true)))))))))))

(fn `UserConstructionScript`)