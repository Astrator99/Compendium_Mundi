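; Game mode that manages pause, input mode and player death and respawn.
; Pausing shows the WBP_Pause widget with cursor and UI-only input; unpausing restores game input.
; On death it fades the camera, clears widgets, destroys the player and respawns either BP_Player or BP_PlayerZD by Is3DMode.
; The spawn transform starts from the player controller and is updatable; respawn also calls PlayerData on GI_GameSettings and fades back in.
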(event `self.ReceiveBeginPlay`
  (bind (_returnvalue_location _returnvalue_rotation _returnvalue_scale) (`KismetMathLibrary.BreakTransform` (`self.GetTransform` (`GameplayStatics.GetPlayerController` 0))))
  (`self.Input UI`)
  (`GameplayStatics.GetActorOfClass` (`self.MeinStartpunkt`))
  (set `self.Spieler Spawnpunkt` (`KismetMathLibrary.MakeTransform` _returnvalue_location _returnvalue_rotation _returnvalue_scale)))

(event `Add Score`
  (set `self.Score` (+ 0 (`self.Score`))))

(event `Input UI`
  (`WidgetBlueprintLibrary.SetInputMode_GameOnly` (`GameplayStatics.GetPlayerController` 0)))

(event `Pause On`
  (bind _returnvalue (`GameplayStatics.GetPlayerController` 0))
  ;[0 0.15 0.136 0.5] Funktion - Pause
  (bind _returnvalue_2 (`|GenericCreateObject` "/Game/Assets-UI/WBP_Pause.WBP_Pause_C"))
  (bind _output_get (set `self.UI Pause` _returnvalue_2))
  (`UserWidget.AddToViewport` _output_get 0)
  (`GameplayStatics.SetGamePaused` true)
  (`WidgetBlueprintLibrary.SetInputMode_UIOnlyEx` _returnvalue null)
  (set `PlayerController.bShowMouseCursor` true _returnvalue))

(event `Pause Off`
  (bind _returnvalue (`GameplayStatics.GetPlayerController` 0))
  ;[0 0.15 0.136 0.5] Funktion - Pause
  (`GameplayStatics.SetGamePaused` false)
  (`WidgetBlueprintLibrary.SetInputMode_GameOnly` _returnvalue)
  (set `PlayerController.bShowMouseCursor` false _returnvalue))

(event `/Game/Blueprints/Funktionen/Interface/BPI_GameManagement.TriggerPlayerDeath`
  (params (DeadPlayerActor :type "Actor Object Reference"))
  ;[0.15 0.05914 0.001037 0.5] Funktion - Player Spawn
  (`PlayerCameraManager.StartCameraFade` :`self` (`GameplayStatics.GetPlayerCameraManager` 0) :`ToAlpha` 1.0 :`Duration` 3.0 :`bHoldWhenFinished` true)
  (`WidgetLayoutLibrary.RemoveAllWidgets`)
  (`self.K2_DestroyActor` DeadPlayerActor)
  (`self.PlayerRespawn`))

(event `/Game/Blueprints/Funktionen/Interface/BPI_GameManagement.SetNewSpawnTransform`
  (params (NewTransform :type "Transform Structure"))
  ;[0.15 0.05914 0.001037 0.5] Funktion - Player Spawn
  (set `self.Spieler Spawnpunkt` (`KismetMathLibrary.MakeTransform` NewTransform_Location NewTransform_Rotation NewTransform_Scale)))

(event `PlayerRespawn`
  (bind _spieler_spawnpunkt (`self.Spieler Spawnpunkt`))
  (bind _spieler_spawnpunkt_2 (`self.Spieler Spawnpunkt`))
  ;[0.15 0.05914 0.001037 0.5] Funktion - Player Spawn
  (if (`self.Is3DMode`)
    (bind _returnvalue (`|SpawnActorFromClass` "/Game/Blueprints/Mechaniken/Players/Player-3D/BP_Player.BP_Player_C" (`KismetMathLibrary.MakeTransform` (.location _spieler_spawnpunkt) (`KismetMathLibrary.MakeRotator` 0.0 0.0 (.yaw (.rotation _spieler_spawnpunkt)))) "Undefined" "MultiplyWithRoot" null null))
    (`Controller.Possess` (`GameplayStatics.GetPlayerController` 0) _returnvalue)
    (else
      (bind _returnvalue_2 (`|SpawnActorFromClass` "/Game/Blueprints/Mechaniken/Players/Player-ZD/BP_Player-ZD.BP_Player-ZD_C" (`KismetMathLibrary.MakeTransform` (.location _spieler_spawnpunkt_2) (`KismetMathLibrary.MakeRotator` 0.0 0.0 (.yaw (.rotation _spieler_spawnpunkt_2)))) "Undefined" "MultiplyWithRoot" null null))
      (message `/Game/Blueprints/Funktionen/Interface/BPI_PlayerManagement.InitializeUI` _returnvalue_2)
      (`Controller.Possess` (`GameplayStatics.GetPlayerController` 0) _returnvalue_2)))
  (bind _asgi_game_settings (cast `/Game/Blueprints/GI_GameSettings` (`GameplayStatics.GetGameInstance`)))
  (`/Game/Blueprints/GI_GameSettings.PlayerData` _asgi_game_settings null)
  (`PlayerCameraManager.StartCameraFade` :`self` (`GameplayStatics.GetPlayerCameraManager` 0) :`FromAlpha` 1.0 :`Duration` 3.0 :`bHoldWhenFinished` true))

(fn `GetSettings`
  (returns (Setting :type "/Game/Blueprints/BP_SaveSettings Object Reference"))
  (return null))

(fn `UserConstructionScript`)