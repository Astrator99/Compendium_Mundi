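; Game instance that owns the game's settings save and can restore the player's saved position.
; On Init it loads the settings slot and applies master, music and SFX volumes through sound mix class overrides, or creates the save and runs a hardware benchmark to set graphics settings.
; It exposes the save object and a write-to-slot event.
; PlayerData reloads the slot and, if LoadingfromSave is set, restores player transform and camera rotation.
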(event `self.ReceiveInit`
  (bind _returnvalue (`GameplayStatics.DoesSaveGameExist` (`self.SettingsSlot`)))
  (if _returnvalue
    (bind _returnvalue_2 (`GameplayStatics.LoadGameFromSlot` (`self.SettingsSlot`)))
    (bind _asbp_save_settings (cast `/Game/Blueprints/BP_SaveSettings` _returnvalue_2))
    (set `self.SettingsSave` _asbp_save_settings)
    (`self.LoadAudioSettings`)
    (else
      (bind _returnvalue_3 (`GameplayStatics.CreateSaveGameObject` "/Game/Blueprints/BP_SaveSettings.BP_SaveSettings_C"))
      (`GameplayStatics.SaveGameToSlot` _returnvalue_3 (`self.SettingsSlot`))
      (set `self.SettingsSave` _returnvalue_3)
      (`self.RunBenchmark`))))

(event `/Game/Blueprints/Funktionen/Interface/BPI_GameManagement.SaveSettings`
  (`GameplayStatics.SaveGameToSlot` (`self.SettingsSave`) (`self.SettingsSlot`)))

(event `self.ReceiveShutdown`)

(event `RunBenchmark`
  (bind _returnvalue (`GameUserSettings.GetGameUserSettings`))
  (`GameUserSettings.RunHardwareBenchmark` _returnvalue 10 1.0 1.0)
  (`GameUserSettings.ApplyHardwareBenchmarkResults` _returnvalue)
  (`GameUserSettings.SaveSettings` _returnvalue))

(event `LoadAudioSettings`
  (bind _settingssave (`self.SettingsSave`))
  (`GameplayStatics.SetSoundMixClassOverride` "/Game/Assets-Audio/SKMix_Master.SKMix_Master" "/Game/Assets-Audio/SK_Master.SK_Master" (`/Game/Blueprints/BP_SaveSettings.MasterVolume` _settingssave))
  (`GameplayStatics.SetSoundMixClassOverride` "/Game/Assets-Audio/SKMix_Musik.SKMix_Musik" "/Game/Assets-Audio/SK_Musik.SK_Musik" (`/Game/Blueprints/BP_SaveSettings.MusikVolume` _settingssave))
  (`GameplayStatics.SetSoundMixClassOverride` "/Game/Assets-Audio/SKMix_Sounds.SKMix_Sounds" "/Game/Assets-Audio/SK_Sounds.SK_Sounds" (`/Game/Blueprints/BP_SaveSettings.SFXVolume` _settingssave)))

(event `PlayerData`
  (params (TargetPlayer :type "Actor Object Reference"))
  (bind _returnvalue (`GameplayStatics.LoadGameFromSlot` (`self.SettingsSlot`)))
  (bind _asbp_save_settings (cast `/Game/Blueprints/BP_SaveSettings` _returnvalue))
  (if (`self.LoadingfromSave`)
    (`Actor.K2_SetActorTransform` TargetPlayer (`/Game/Blueprints/BP_SaveSettings.SpielerPosition` _asbp_save_settings) false false)
    (`Controller.SetControlRotation` (`GameplayStatics.GetPlayerController` 0) (`/Game/Blueprints/BP_SaveSettings.SpielerKameraRotierung` _asbp_save_settings))))

(fn `GetSettings`
  (returns (Setting :type "/Game/Blueprints/BP_SaveSettings Object Reference"))
  (return (`self.SettingsSave`)))